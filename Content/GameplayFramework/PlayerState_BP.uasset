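; Player state Blueprint that holds the player's health and armor and flags game over when health runs out.
; Its construction script loads Health, MaxHealth and MaxArmor from the default row of the PlayerSettings_Table data table.
; ChangeHealth scales damage down by current Armor and, at zero health, sets GameOver on GameMode_BP.
; Non-negative changes use Max against MaxHealth, so they raise Health to at least MaxHealth rather than capping it.
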(fn `ChangeHealth`
  (params (HealthIncrement :type "Float (double-precision)"))
  (bind _health (`self.Health`))
  ;[0.0744 0.0744 0.0744] Обрабатывает изменение здоровья игрока, если оно становится равным 0 - устанавливает окончание игры в GameMode
  (if (< HealthIncrement 0.0)
    (bind _output_get (set `self.Health` (+ (* HealthIncrement (- 1.0 (* (`self.Armor`) 0.2))) _health)))
    (if (<= _output_get 0.0)
      (set `self.Health` 0.0)
      (bind _asgame_mode_bp (cast `/Game/GameplayFramework/GameMode_BP` (`GameplayStatics.GetGameMode`)))
      (set `/Game/GameplayFramework/GameMode_BP.GameOver` true _asgame_mode_bp))
    (else
      (set `self.Health` (`KismetMathLibrary.FMax` (+ HealthIncrement _health) (`self.MaxHealth`))))))

(fn `UserConstructionScript`
  (bind _returnvalue (`|GetDataTableRow` "/Game/Settings/PlayerSettings/PlayerSettings_Table.PlayerSettings_Table" "DefaultSettings")
    (:`then`
      (bind _output_get (set `self.Health` (break `/Game/Settings/PlayerSettings/PlayerSettings_Struct` _returnvalue)))
      (set `self.MaxHealth` _output_get)
      (set `self.MaxArmor` (`.MaxArmor_5_A4EB1AD940EF4A07DA2916B2D0A675A4` (break `/Game/Settings/PlayerSettings/PlayerSettings_Struct` _returnvalue))))))