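; Bullet_BP is a projectile actor that reacts physically, audibly and visually when it hits something.
; On Hit, it pushes physics-simulating components with an impulse taken from its velocity, applied at the bullet's location.
; It then plays a rifle impact sound, spawns a muzzle flash particle effect as the impact visual, and destroys itself.
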(event `self.ReceiveBeginPlay`
  (`PrimitiveComponent.IgnoreActorWhenMoving` (`self.ParticleSystem`) null false))

(event `self.ReceiveHit`
  (params (MyComp :type "PrimitiveComponent Object Reference") (Other :type "Actor Object Reference") (OtherComp :type "PrimitiveComponent Object Reference") (bSelfMoved :type Boolean) (HitLocation :type "Vector Structure") (HitNormal :type "Vector Structure") (NormalImpulse :type "Vector Structure") (Hit :type "HitResult Structure (by ref)"))
  (bind _returnvalue (`self.K2_GetActorLocation`))
  ;[1 1 1] Hit logic
  (if (`SceneComponent.IsSimulatingPhysics` OtherComp "None")
    (`PrimitiveComponent.AddImpulseAtLocation` OtherComp (* (`self.GetVelocity`) 1.0) (`self.K2_GetActorLocation`) "None"))
  (`GameplayStatics.PlaySoundAtLocation` "/Game/MilitaryWeapSilver/Sound/Rifle/Wavs/Rifle_ImpactSurface01.Rifle_ImpactSurface01" _returnvalue (struct) 1.0 1.0 0.0 null null null null)
  (`GameplayStatics.SpawnEmitterAtLocation` "/Game/MilitaryWeapSilver/FX/P_AssaultRifle_MuzzleFlash.P_AssaultRifle_MuzzleFlash" _returnvalue)
  (`self.K2_DestroyActor`) ; Then destroy this projectile
)

(fn `UserConstructionScript`)