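; HUD Blueprint that creates and shows the player's on-screen widgets for health, armor, details count, aim and tasks.
; BeginPlay caches the custom PlayerState, GameMode and GameState, then creates each widget and adds it to the viewport.
; DrawHUD refreshes health from the cached PlayerState and tells the armor widget to update every frame, while the other widgets receive no updates here.
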(event `self.ReceiveDrawHUD`
  (params (SizeX :type Integer) (SizeY :type Integer))
  (`/Game/UI/HealthWidget/HealthWidget_BP.UpdateHealth` (`self.HealthWidget`) (`/Game/GameplayFramework/PlayerState_BP.Health` (`self.PlayerState`)))
  (`/Game/UI/ArmorWidget/ArmorWidget_BP.UpdateArmor` (`self.ArmorWidget`)))

(event `self.ReceiveBeginPlay`
  ;[0.2122 0.2122 0.2122 0.498] Data init
  (bind _asplayer_state_bp (cast `/Game/GameplayFramework/PlayerState_BP` (`GameplayStatics.GetPlayerState` 0)))
  (set `self.PlayerState` _asplayer_state_bp)
  (bind _asgame_mode_bp (cast `/Game/GameplayFramework/GameMode_BP` (`GameplayStatics.GetGameMode`)))
  (set `self.GameMode` _asgame_mode_bp)
  (bind _asgame_state_bp (cast `/Game/GameplayFramework/GameState_BP` (`GameplayStatics.GetGameState`)))
  (set `self.GameState` _asgame_state_bp)
  (bind _returnvalue (`|CreateWidget` "/Game/UI/HealthWidget/HealthWidget_BP.HealthWidget_BP_C"))
  (bind _output_get (set `self.HealthWidget` _returnvalue))
  (`UserWidget.AddToViewport` _output_get 0)
  (bind _returnvalue_2 (`|CreateWidget` "/Game/UI/DetailsCountWidget/DetailsCountWidget_BP.DetailsCountWidget_BP_C"))
  (bind _output_get_2 (set `self.DetailsCountWidget` _returnvalue_2))
  (`UserWidget.AddToViewport` _output_get_2 0)
  (bind _returnvalue_3 (`|CreateWidget` "/Game/MilitaryWeapSilver/HUD_Aim.HUD_Aim_C"))
  (bind _output_get_3 (set `self.AimWidget` _returnvalue_3))
  (`UserWidget.AddToViewport` _output_get_3 0)
  (bind _returnvalue_4 (`|CreateWidget` "/Game/UI/ArmorWidget/ArmorWidget_BP.ArmorWidget_BP_C"))
  (bind _output_get_4 (set `self.ArmorWidget` _returnvalue_4))
  (`UserWidget.AddToViewport` _output_get_4 0)
  (bind _returnvalue_5 (`|CreateWidget` "/Game/UI/TaskWidget/TaskWidget_BP.TaskWidget_BP_C"))
  (bind _output_get_5 (set `self.TaskWidget` _returnvalue_5))
  (`UserWidget.AddToViewport` _output_get_5 0))

(fn `UserConstructionScript`)