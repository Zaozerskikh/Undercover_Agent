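; Mission manager actor that holds a list of missions and tracks which one is current.
; Added missions join the list, and the first becomes current if none is.
; SetCurrentMission swaps states and state-change bindings, fires a change notification and refreshes the HUD task widget.
; A mission's end state triggers removal and selection of the first listed mission, but RemoveMissionByPointer's removal logic is disconnected, so nothing leaves the list.
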(event `OnChangedStateMission`
  (params (InMission :type "/Game/MissionSystem/BP_Mission Object Reference") (InNewState :type "/Game/MissionSystem/MissionStatus_Enum Enum" :default "NewEnumerator0"))
  (bind _missions (`self.Missions`))
  (if (`|EnumEquality` InNewState "NewEnumerator2")
    (`self.RemoveMissionByPointer` InMission)
    (if (`KismetArrayLibrary.Array_IsNotEmpty` _missions)
      (`self.SetCurrentMission` (`|GetArrayItem` _missions)))))

(fn `Add Next Mission`
  (params (InMission :type "/Game/MissionSystem/BP_Mission Object Reference"))
  (`KismetArrayLibrary.Array_Add` (`self.Missions`) InMission)
  (`/Game/MissionSystem/BP_Mission.UpdateState` InMission "NewEnumerator1")
  (`/Engine/EditorBlueprintResources/StandardMacros.IsValid` (`self.CurrentMission`)
    (:`Is Not Valid`
      (`self.SetCurrentMission` (`local.InMission`)))))

(fn `RemoveAllMissions`
  (`self.SetCurrentMission` null)
  (`KismetArrayLibrary.Array_Clear` (`self.Missions`)))

(fn `RemoveMissionByPointer`
  (params (InMission :type "/Game/MissionSystem/BP_Mission Object Reference"))
  (`/Engine/EditorBlueprintResources/StandardMacros.IsValid` InMission))

(fn `SetCurrentMission`
  (params (InMission :type "/Game/MissionSystem/BP_Mission Object Reference"))
  (bind _currentmission (`self.CurrentMission`))
  (bind _inmission (`local.InMission`))
  (if (!= InMission (`self.CurrentMission`))
    (`/Engine/EditorBlueprintResources/StandardMacros.IsValid` _currentmission
      (:`Is Valid`
        (remove `/Game/MissionSystem/BP_Mission.OnChangedStateMission` _currentmission (`|CreateDelegate` :!event `OnChangedStateMission`))
        (if (`|EnumInequality` (`/Game/MissionSystem/BP_Mission.State` (`self.CurrentMission`)) "NewEnumerator2")
          (`/Game/MissionSystem/BP_Mission.UpdateState` (`self.CurrentMission`) "NewEnumerator1"))
        (set `self.CurrentMission` null))
      (:`Is Not Valid`
        _))
    (`/Engine/EditorBlueprintResources/StandardMacros.IsValid` _inmission
      (:`Is Valid`
        (bind _output_get (set `self.CurrentMission` _inmission))
        (`/Game/MissionSystem/BP_Mission.UpdateState` _output_get "NewEnumerator0")
        (add `/Game/MissionSystem/BP_Mission.OnChangedStateMission` _output_get (`|CreateDelegate` :!event `OnChangedStateMission`)))
      (:`Is Not Valid`
        _))
    (`self.OnChangedCurrentMission` (`self.CurrentMission`))
    (bind _ashud_bp (cast `/Game/GameplayFramework/HUD_BP` (`PlayerController.GetHUD` (`GameplayStatics.GetPlayerController` 0))))
    (`/Game/UI/TaskWidget/TaskWidget_BP.UpdateTask` (`/Game/GameplayFramework/HUD_BP.TaskWidget` _ashud_bp))))

(fn `UserConstructionScript`)