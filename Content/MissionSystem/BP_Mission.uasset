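; BP_Mission is a mission actor that holds one mission's info, owning player character, phase and current state.
; Init stores the supplied info and character, then resets the phase to zero.
; UpdateState prints a message with the mission name, sets the new state and broadcasts it with itself through the OnChangedStateMission dispatcher.
; The event graph and construction script are empty, so both functions rely on external callers.
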(fn `Init`
  (params (InMissionInfo :type "/Game/MissionSystem/Missions_Structure Structure") (InPlayerCharacter :type "/Game/GameplayFramework/PlayerCharacter_BP Object Reference"))
  (set `self.Info` InMissionInfo)
  (set `self.OwnerPlayerCharacter` InPlayerCharacter)
  (set `self.Phase` 0))

(fn `UpdateState`
  (params (InNewState :type "/Game/MissionSystem/MissionStatus_Enum Enum" :default "NewEnumerator0"))
  (bind (_info_name _info_numphases _info_nameui) (break `/Game/MissionSystem/Missions_Structure` (`self.Info`)))
  (`KismetSystemLibrary.PrintString` (`KismetStringLibrary.Concat_StrStr` (`KismetTextLibrary.Conv_TextToString` _info_nameui) "changed status to '" (`|GetEnumeratorNameAsString` (`local.InNewState`)) "'"))
  (bind _output_get (set `self.State` (`local.InNewState`)))
  (`self.OnChangedStateMission` self _output_get))

(fn `UserConstructionScript`)