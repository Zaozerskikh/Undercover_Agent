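; BP_Spawner_10 is a spawner actor that continuously spawns Monster_BP at its own transform, starting on BeginPlay.
; The Spawn event creates a monster, adjusting for collisions but always spawning, waits for the Delay variable, then calls itself, looping with no count limit.
; A GetSpawnLocation stub returning zero and a random navigable-point lookup using Radius are left unused.
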(event `self.ReceiveBeginPlay`
  (`self.Spawn`))

(event `Spawn`
  (`|SpawnActorFromClass` "/Game/ThirdPerson/Blueprints/Monster/Monster_BP.Monster_BP_C" (`self.GetTransform`) "AdjustIfPossibleButAlwaysSpawn" "OverrideRootScale" null null)
  (`KismetSystemLibrary.Delay` (`self.Delay`))
  (`self.Spawn`))

(fn `GetSpawnLocation`
  (returns (Location :type "Vector Structure"))
  (return (0.0 0.0 0.0)))

(fn `UserConstructionScript`)