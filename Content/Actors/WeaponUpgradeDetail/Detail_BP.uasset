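; Detail_BP is a weapon-upgrade detail pickup that the player collects by overlapping it.
; The Heart_rotation timeline starts on BeginPlay and spins the root around yaw.
; On overlap with PlayerCharacter_BP, it increments DetailsCount in GameInstance_BP and destroys itself.
; The construction script reads HealthIncrement from the "Basic" row of HealthPickupSettingsTable, but the pickup logic never uses it.
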(event `self.ReceiveBeginPlay`
  ;[0.2122 0.2122 0.2122 0.498] Rotation
  (bind (_direction _newtrack_0) (`Timeline|heart_rotation`)
    (:`Update`
      (`SceneComponent.K2_AddRelativeRotation` (`self.DefaultSceneRoot`) (`KismetMathLibrary.MakeRotator` 0.0 0.0 _newtrack_0) false false))))

(event `self.ReceiveActorBeginOverlap`
  (params (OtherActor :type "Actor Object Reference"))
  ;[0.2122 0.2122 0.2122 0.498] Collision
  (cast `/Game/GameplayFramework/PlayerCharacter_BP` OtherActor)
  (bind _asgame_instance_bp (cast `/Game/GameplayFramework/GameInstance_BP` (`GameplayStatics.GetGameInstance`)))
  (set `/Game/GameplayFramework/GameInstance_BP.DetailsCount` (+ (`/Game/GameplayFramework/GameInstance_BP.DetailsCount` _asgame_instance_bp) 1) _asgame_instance_bp)
  (`self.K2_DestroyActor`))

(fn `UserConstructionScript`
  (bind _returnvalue (`|GetDataTableRow` "/Game/Settings/UpgradeSystemSettings/HealthPickupSettings/HealthPickupSettingsTable.HealthPickupSettingsTable" "Basic")
    (:`then`
      (set `self.HealthIncrement` (break `/Game/Settings/UpgradeSystemSettings/HealthPickupSettings/HealthPickupSettings_Struct` _returnvalue)))))